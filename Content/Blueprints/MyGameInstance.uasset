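; Game instance Blueprint that handles hosting and joining multiplayer sessions.
; HOST_GAME creates a session for the first player controller, then opens GameMap as a listen server, adding the LAN match option when LAN is requested.
; JOIN joins a given search result.
; Both events print success or failure messages.
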(event `HOST_GAME`
  (params (PublicConnections :type Integer) (bUseLAN :type Boolean))
  (`CreateSessionCallbackProxy.CreateSession` (`GameplayStatics.GetPlayerController` 0) PublicConnections bUseLAN
    (:`OnSuccess`
      (`KismetSystemLibrary.PrintString` "Session created")
      (if bUseLAN
        (`GameplayStatics.OpenLevel` "GameMap" true "listen?bIsLanMatch=1")
        (else
          (`GameplayStatics.OpenLevel` "GameMap" true "listen"))))
    (:`OnFailure`
      (`KismetSystemLibrary.PrintString` "Failed to create session"))))

(event `JOIN`
  (params (SearchResult :type "BlueprintSessionResult Structure (by ref)"))
  (`JoinSessionCallbackProxy.JoinSession` (`GameplayStatics.GetPlayerController` 0) SearchResult
    (:`OnSuccess`
      (`KismetSystemLibrary.PrintString` "Session Joined"))
    (:`OnFailure`
      (`KismetSystemLibrary.PrintString` "Failed to join session"))))